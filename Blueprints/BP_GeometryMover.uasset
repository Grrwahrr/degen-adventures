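; BP_GeometryMover is an actor that scrolls its geometry vertically in a loop, staying idle until activated.
; ActivateGeometryMover sets the IsActive flag, after which Tick moves the root component along world Z at Speed, scaled by delta time.
; Once its height exceeds ResetIfZGreaterThan, it snaps back to RespawnAtZLoc while keeping X and Y, giving a treadmill-style repeat.
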(event EventTick
  (params (DeltaSeconds :type Float%20%28single-precision%29))
  (bind _defaultsceneroot (Variables|Default|GetDefaultSceneRoot))
  (bind _returnvalue (Transformation|GetWorldLocation _defaultsceneroot))
  (if (Variables|MoveableGeometry|GetIsActive)
    (Transformation|SetWorldLocation _defaultsceneroot (Math|Vector|MakeVector (.x _returnvalue) (.y _returnvalue) (+ (* DeltaSeconds (Variables|MoveableGeometry|GetSpeed)) (.z _returnvalue))) false false)
    (if (> (.z (Transformation|GetWorldLocation (Variables|Default|GetDefaultSceneRoot))) (Variables|MoveableGeometry|GetResetIfZGreaterThan))
      (Transformation|SetWorldLocation (Variables|Default|GetDefaultSceneRoot) (Math|Vector|MakeVector (.x _returnvalue) (.y _returnvalue) (Variables|MoveableGeometry|GetRespawnAtZLoc)) false false))))

(fn ConstructionScript)

(fn ActivateGeometryMover
  (Variables|MoveableGeometry|SetIsActive true))