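; Robo Gensler boss that, once triggered, rides its Speeder along a spline and attacks the BP_Bonk player character.
; Tick advances spline distance, with a Delay governing loop reset or stop.
; A looping timer randomly spawns regulation attacks into a stack, then launches them together at scattered points around the player once stack size and cooldown allow.
; The required stack size randomly grows during the fight, and taunts accompany trigger and volleys.
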(event EventBeginPlay)

(event Collision|EventActorBeginOverlap
  (params (OtherActor :type Actor%20Object%20Reference)))

(event EventTick
  (params (DeltaSeconds :type Float%20%28single-precision%29))
  (bind _speeder (Variables|Default|GetSpeeder))
  (if (Variables|RoboSpeeder|GetWasTriggered)
    (bind _output_get (Variables|RoboSpeeder|SetDistance (+ (* DeltaSeconds (Variables|RoboSpeeder|GetSpeed)) (Variables|RoboSpeeder|GetDistance) 1.0)))
    (Transformation|SetRelativeTransform _speeder (Math|Transform|MakeTransform (.location (Spline|GetTransformatDistanceAlongSpline (Variables|Default|GetSpline) _output_get "Local" false)) (Math|Rotator|MakeRotator (.roll (.rotation (Spline|GetTransformatDistanceAlongSpline (Variables|Default|GetSpline) _output_get "Local" false))) (.pitch (.rotation (Spline|GetTransformatDistanceAlongSpline (Variables|Default|GetSpline) _output_get "Local" false))) (+ (.yaw (.rotation (Spline|GetTransformatDistanceAlongSpline (Variables|Default|GetSpline) _output_get "Local" false))) -9e+01)) (Variables|/Script/Engine.SceneComponent|GetRelativeScale3D _speeder)) false false)
    (Utilities|FlowControl|Delay (Variables|RoboSpeeder|GetDuration))
    (if (Variables|Default|GetIslooping)
      (Variables|RoboSpeeder|SetDistance 1.0)
      (else
        (Variables|RoboSpeeder|SetWasTriggered false)))))

(fn ConstructionScript)

(fn TriggerGensler
  (Variables|RoboSpeeder|SetWasTriggered true)
  (Utilities|Time|SetTimerbyFunctionName 0 "AttackTimer" (Variables|RoboSpeeder|GetAttackInterval) true false 5.0)
  (bind _asbp_bonk (Utilities|Casting|CastToBP_Bonk (Game|GetPlayerCharacter 0)))
  (Variables|RoboSpeederInternal|SetTheBonk _asbp_bonk)
  (Audio|PlaySound2D "/Game/ThirdPerson/SFX/Gensler/BossTaunts.BossTaunts" 9.0 1.0 0.0 0 0))

(fn AttackTimer
  (bind _thebonk (Variables|RoboSpeederInternal|GetTheBonk))
  (bind _attackstack (Variables|RoboSpeederInternal|GetAttackStack))
  (bind _robo (Variables|Default|GetRobo))
  (bind _returnvalue (Transformation|GetWorldLocation _robo))
  (bind _capsulecomponent (Variables|/Script/Engine.Character|GetCapsuleComponent _thebonk))
  (bind _returnvalue_2 (Transformation|GetWorldLocation _capsulecomponent))
  (Variables|RoboSpeederInternal|SetAssaultTimeAccumulator (+ (Variables|RoboSpeeder|GetAttackInterval) (Variables|RoboSpeederInternal|GetAssaultTimeAccumulator)))
  (Utilities|IsValid _thebonk
    (:Is%20Valid
      (if (> (Math|Random|RandomIntegerinRange 0 1000) 750)
        (Utilities|FlowControl|Sequence
          (:then_0
            (Variables|RoboSpeederInternal|SetAttackCounter (+ (Variables|RoboSpeederInternal|GetAttackCounter) 1))
            (if (> (Math|Random|RandomIntegerinRange 0 1000) 750)
              (Variables|RoboSpeederInternal|SetAttackAtStackSize (+ (Variables|RoboSpeederInternal|GetAttackAtStackSize) 1))))
          (:then_1
            (bind _returnvalue_3 (Game|SpawnActorfromClass "/Game/ThirdPerson/Blueprints/BP_RegulationAttack.BP_RegulationAttack_C" (Math|Transform|MakeTransform (+ _returnvalue (Math|Vector|MakeVector 0.0 0.0 (Math|Random|RandomFloatinRange -2e+02 2e+02))) (Math|Rotator|FindLookatRotation _returnvalue _returnvalue_2) "1.000000,1.000000,1.000000") "AlwaysSpawn" "MultiplyWithRoot" 0 0))
            (Utilities|Array|Add (Variables|RoboSpeederInternal|GetAttackStack) _returnvalue_3))
          (:then_2
            (if (and (>= (Utilities|Array|Length (Variables|RoboSpeederInternal|GetAttackStack)) (Variables|RoboSpeederInternal|GetAttackAtStackSize)) (> (Variables|RoboSpeederInternal|GetAssaultTimeAccumulator) (Variables|RoboSpeeder|GetMinTimeBetweenAssaults)))
              (Variables|RoboSpeederInternal|SetAssaultTimeAccumulator 0.0)
              (Audio|PlaySound2D "/Game/ThirdPerson/SFX/Gensler/BossTaunts.BossTaunts" 7.0 1.0 0.0 0 0 false)
              (for _array_element _attackstack
                (Default|EngageTargetLocation _array_element (+ _returnvalue_2 (Math|Vector|MakeVector (Math|Random|RandomFloatinRange -2e+02 2e+02) 0.0 (Math|Random|RandomFloatinRange -2e+02 2e+02))) 4.5e+02))
              (Utilities|Array|Clear _attackstack))))))))