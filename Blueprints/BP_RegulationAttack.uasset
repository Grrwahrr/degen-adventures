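; BP_RegulationAttack is a projectile attack that costs BP_Bonk a life on contact.
; EngageTargetLocation turns the collision box toward a target location, launches ProjectileMovement at the given speed, sets the player capsule as homing target and limits the lifespan.
; Overlapping a BP_Bonk destroys the projectile, calls BonkLostLive without respawn and plays a hit sound.
; Tick is empty, and a manual movement branch is left unconnected.
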(event OnComponentBeginOverlap(CollisionBox)
  (params (OverlappedComponent :type Primitive%20Component%20Object%20Reference) (OtherActor :type Actor%20Object%20Reference) (OtherComp :type Primitive%20Component%20Object%20Reference) (OtherBodyIndex :type Integer) (bFromSweep :type Boolean) (SweepResult :type Hit%20Result%20Structure%20%28by%20ref%29))
  (bind _asbp_bonk (Utilities|Casting|CastToBP_Bonk OtherActor))
  (Actor|DestroyActor)
  (Default|BonkLostLive _asbp_bonk false 0.0)
  (Audio|PlaySound2D "/Game/ThirdPerson/SFX/SFX_AttackHit.SFX_AttackHit" 2.0 1.0 0.0 0 0))

(event EventTick
  (params (DeltaSeconds :type Float%20%28single-precision%29)))

(fn ConstructionScript)

(fn EngageTargetLocation
  (params (TargetLocation :type Vector) (Speed :type Float%20%28double-precision%29))
  (bind _collisionbox (Variables|Default|GetCollisionBox))
  (bind _projectilemovement (Variables|Default|GetProjectileMovement))
  (bind _returnvalue (Transformation|GetWorldLocation _collisionbox))
  (Transformation|SetWorldLocationAndRotation (Variables|Default|GetCollisionBox) _returnvalue (Math|Rotator|FindLookatRotation _returnvalue TargetLocation) false false)
  (Variables|/Script/Engine.MovementComponent|SetVelocity _projectilemovement (* (Math|Vector|GetForwardVector (Variables|Default|GetCollisionBox)) Speed))
  (Variables|/Script/Engine.ProjectileMovementComponent|SetHomingTargetComponent _projectilemovement (Variables|/Script/Engine.Character|GetCapsuleComponent (Game|GetPlayerCharacter 0)))
  (Actor|SetLifeSpan 1e+01))