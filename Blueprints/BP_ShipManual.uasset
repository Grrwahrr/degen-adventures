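; BP_ShipManual is an actor that flies a ship mesh along a spline once ActivateFlyingShip sets its trigger flag.
; Tick advances distance by Speed times delta plus one unit per frame, then applies the spline's local location and rotation to the mesh.
; A Delay of Duration, rather than spline length, decides when the flight restarts if looping or otherwise stops.
; The Construction Script holds only an empty segment loop with unused spline nodes.
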(event EventBeginPlay)

(event EventTick
  (params (DeltaSeconds :type Float%20%28single-precision%29))
  (bind _sm_ship (Variables|Default|GetSM_ship))
  (if (Variables|FlyingShip|GetWasTriggered)
    (bind _output_get (Variables|FlyingShip|SetDistance (+ (* DeltaSeconds (Variables|FlyingShip|GetSpeed)) (Variables|FlyingShip|GetDistance) 1.0)))
    (Transformation|SetRelativeTransform _sm_ship (Math|Transform|MakeTransform (.location (Spline|GetTransformatDistanceAlongSpline (Variables|Default|GetSpline) _output_get "Local" false)) (.rotation (Spline|GetTransformatDistanceAlongSpline (Variables|Default|GetSpline) _output_get "Local" false)) (Variables|/Script/Engine.SceneComponent|GetRelativeScale3D _sm_ship)) false false)
    (Utilities|FlowControl|Delay (Variables|FlyingShip|GetDuration))
    (if (Variables|FlyingShip|GetIslooping)
      (Variables|FlyingShip|SetDistance 1.0)
      (else
        (Variables|FlyingShip|SetWasTriggered false)))))

(fn ConstructionScript
  (for _index (range 0 (- (Math|Float|Truncate (/ (Spline|GetSplineLength (Variables|Default|GetSpline)) (Variables|FlyingShip|GetLength))) 1))
    _))

(fn ActivateFlyingShip
  (Variables|FlyingShip|SetWasTriggered true))