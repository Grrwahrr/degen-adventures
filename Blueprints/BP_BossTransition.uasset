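; BP_BossTransition is a trigger volume that moves the player, BP_Bonk, into the boss fight.
; On overlap it plays dark-fire distortion and sound, fades the camera out and disables input for the transition time.
; It then destroys the old room, teleports Bonk to a hard-coded location, activates the new room's geometry movers, restores input and view, and triggers Gensler.
; Everything after the delay runs only if the room to delete is still valid.
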(event OnComponentBeginOverlap(ColissionBox)
  (params (OverlappedComponent :type Primitive%20Component%20Object%20Reference) (OtherActor :type Actor%20Object%20Reference) (OtherComp :type Primitive%20Component%20Object%20Reference) (OtherBodyIndex :type Integer) (bFromSweep :type Boolean) (SweepResult :type Hit%20Result%20Structure%20%28by%20ref%29))
  (bind _gensler (Variables|TransitionSettings|GetGensler))
  (bind _deleteroom (Variables|TransitionSettings|GetDeleteRoom))
  (bind _transitiontime (Variables|TransitionSettings|GetTransitionTime))
  (bind _asbp_bonk (Utilities|Casting|CastToBP_Bonk OtherActor))
  (Niagara|SpawnSystemAttached "/Game/Fire_Spells_Traps_VFXpack/Particles/P_DarkFire_Distortion.P_DarkFire_Distortion" (Variables|Default|GetDefaultSceneRoot) "None" "0, 0, 0" "0, 0, 0" "KeepRelativeOffset" false)
  (Audio|PlaySound2D "/Game/ThirdPerson/SFX/SFX_BossTransition.SFX_BossTransition" 2.0 1.0 0.0 0 0)
  (CameraFades|StartCameraFade :self (Game|GetPlayerCameraManager 0) :ToAlpha 1.0 :Duration _transitiontime)
  (Input|DisableInput _asbp_bonk (Game|GetPlayerController 0))
  (Utilities|FlowControl|Delay _transitiontime)
  (Utilities|IsValid _deleteroom
    (:Is%20Valid
      (Actor|DestroyActor _deleteroom)
      (Transformation|Teleport _asbp_bonk "70250.000000,4240.000000,780.000000" "0, 0, 0")
      (for _array_element (Variables|TransitionSettings|GetEnableRoomMotion)
        (Utilities|IsValid _array_element
          (:Is%20Valid
            (Default|ActivateGeometryMover _array_element))))
      (Input|EnableInput _asbp_bonk (Game|GetPlayerController 0))
      (CameraFades|StopCameraFade (Game|GetPlayerCameraManager 0))
      (Utilities|IsValid _gensler
        (:Is%20Valid
          (Default|TriggerGensler _gensler))))))

(event EventBeginPlay)

(event Collision|EventActorBeginOverlap
  (params (OtherActor :type Actor%20Object%20Reference)))

(event EventTick
  (params (DeltaSeconds :type Float%20%28single-precision%29)))

(fn ConstructionScript)