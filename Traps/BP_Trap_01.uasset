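; BP_Trap_01 is a cyclic hazard trap that makes BP_Bonk lose a life on overlapping its capsule while active.
; A self-restarting timeline plays forward, holds briefly, reverses, then pauses before repeating, driving Niagara power and the mesh's texture glow parameter together.
; The capsule is harmless only during the pause after reversal, when the effect is deactivated.
; A second timeline for a variant with warning is present but never runs.
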(event OnComponentBeginOverlap(Capsule)
  (params (OverlappedComponent :type Primitive%20Component%20Object%20Reference) (OtherActor :type Actor%20Object%20Reference) (OtherComp :type Primitive%20Component%20Object%20Reference) (OtherBodyIndex :type Integer) (bFromSweep :type Boolean) (SweepResult :type Hit%20Result%20Structure%20%28by%20ref%29))
  (bind _asbp_bonk (Utilities|Casting|CastToBP_Bonk OtherActor))
  (if (not (Variables|Default|GetIsPaused))
    (Default|BonkLostLive _asbp_bonk false 0.0)))

(event Custom|Again
  (bind _niagaratrap (Variables|Default|GetNiagaraTrap))
  (Components|Activation|Activate _niagaratrap true)
  (Components|Timeline|SetPlayRate (Variables|Default|GetTimeline_0) 1.0)
  ;[1 1 1] Trap without warning
  (Variables|Default|SetIsPaused false)
  (bind (_direction _power _texture_boost) (Timeline|Timeline_0 PlayFromStart)
    (:Update
      (Effects|Components|ParticleSystem|SetFloatParameter _niagaratrap "User.Power" _power)
      (Rendering|Material|SetScalarParameterValueonMaterials (Variables|Default|GetTrap) "Texture_Power" _texture_boost))
    (:Finished
      (if (Utilities|Enum|Equal(Enum) _direction "Forward")
        (Utilities|FlowControl|Delay 0.5)
        (CallFunction|Reverse)
        (else
          (Components|Activation|Deactivate (Variables|Default|GetNiagaraTrap))
          (Variables|Default|SetIsPaused true)
          (Utilities|FlowControl|Delay 1.0)
          (CallFunction|Again))))))

(event Custom|Reverse
  ;[1 1 1] Trap without warning
  (Components|Timeline|SetPlayRate (Variables|Default|GetTimeline_0) 1.0)
  (bind (_direction _power _texture_boost) (Timeline|Timeline_0 ReverseFromEnd)
    (:Update
      (Effects|Components|ParticleSystem|SetFloatParameter (Variables|Default|GetNiagaraTrap) "User.Power" _power)
      (Rendering|Material|SetScalarParameterValueonMaterials (Variables|Default|GetTrap) "Texture_Power" _texture_boost))
    (:Finished
      (if (Utilities|Enum|Equal(Enum) _direction "Forward")
        (Utilities|FlowControl|Delay 0.5)
        (CallFunction|Reverse)
        (else
          (Components|Activation|Deactivate (Variables|Default|GetNiagaraTrap))
          (Variables|Default|SetIsPaused true)
          (Utilities|FlowControl|Delay 1.0)
          (CallFunction|Again))))))

(event EventBeginPlay
  (CallFunction|Again))

(fn ConstructionScript)